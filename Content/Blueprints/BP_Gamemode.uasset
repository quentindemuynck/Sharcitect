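; Tower defense game mode that runs enemy waves, awards coins when a wave ends and decides victory or defeat.
; It constructs a BP_WaveManager and polls it on Tick to queue the current wave, which a looping timer spawns at the spawn point.
; Emptied queued and alive lists mark wave end.
; All waves cleared or a dead home base triggers DisableAll, destroying enemies and halting turrets and bullets.
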(event Custom|SpawnEnemies
  (Utilities|Time|SetTimerbyEvent (delegate Custom|SpawnEnemies) (.spawndelay (Variables|Default|GetCurrentWave)) true)
  (if (Math|Conversions|ToBoolean(Integer) (Utilities|Array|Length (Variables|Default|GetQueuedEnemies)))
    ;[1 1 1] Spawn enemies and add them to the alive enemies
    (bind _returnvalue (Game|SpawnActorfromClass (Utilities|Array|Get(acopy) (Variables|Default|GetQueuedEnemies)) (Transformation|GetActorTransform (Variables|/Script/MyProject.WaveManager|GetbM_SpawnLocation (Variables|Default|GetWaveManager))) "Undefined" "MultiplyWithRoot" 0 0))
    (Utilities|Array|RemoveIndex (Variables|Default|GetQueuedEnemies))
    (Utilities|Array|Add (Variables|Default|GetAliveEnemies) _returnvalue)))

(event Custom|DisableAll
  (bind _outactors (Actor|GetAllActorsOfClass "/Game/Blueprints/Enemies/BP_BaseEnemy.BP_BaseEnemy_C"))
  (for _array_element _outactors
    (Actor|DestroyActor _array_element))
  (bind _outactors_2 (Actor|GetAllActorsOfClass "/Game/Blueprints/Turrets/BP_BaseTurrtC.BP_BaseTurrtC_C"))
  (for _array_element_2 _outactors_2
    (Variables|/Game/Blueprints/Turrets/BP_BaseTurrtC.BP_BaseTurrtC_C|SetEnabled _array_element_2 true)
    (Actor|Tick|SetActorTickEnabled _array_element_2))
  (bind _outactors_3 (Actor|GetAllActorsOfClass "/Game/Blueprints/Turrets/BP_Bullet.BP_Bullet_C"))
  (for _array_element_3 _outactors_3
    (Actor|Tick|SetActorTickEnabled _array_element_3))
  (bind _outactors_4 (Actor|GetAllActorsOfClass "/Game/Blueprints/Shields/BP_BaseShield.BP_BaseShield_C"))
  (for _array_element_4 _outactors_4
    (Variables|/Game/Blueprints/Shields/BP_BaseShield.BP_BaseShield_C|SetEnabled _array_element_4 true)
    (Actor|Tick|SetActorTickEnabled _array_element_4 true))
  (Variables|Default|SetAlreadyDisabled true))

(event EventBeginPlay
  (bind _returnvalue (Game|ConstructObjectfromClass "/Game/Blueprints/WaveManager/BP_WaveManager.BP_WaveManager_C"))
  (bind _output_get (Variables|Default|SetWaveManager _returnvalue))
  (bind _returnvalue_2 (Actor|GetActorOfClass "/Game/Blueprints/WaveManager/BP_EnemySpawnPoint.BP_EnemySpawnPoint_C"))
  (bind _output_get_2 (Variables|/Script/MyProject.WaveManager|SetbM_SpawnLocation _output_get _returnvalue_2))
  (Development|PrintString (Utilities|GetDisplayName _output_get_2))
  (bind _returnvalue_3 (Actor|GetActorOfClass "/Game/Blueprints/BP_HomeBase.BP_HomeBase_C"))
  (Variables|Default|SetBase _returnvalue_3)
  (bind _asbp_game_instance (Utilities|Casting|CastToBP_GameInstance (Game|GetGameInstance)))
  (Variables|Default|SetGameInstance _asbp_game_instance))

(event EventTick
  (params (DeltaSeconds :type Float%20%28single-precision%29))
  (bind _gameinstance (Variables|Default|GetGameInstance))
  (if (Variables|/Script/MyProject.WaveManager|GetbM_IsPlayingWave (Variables|Default|GetWaveManager))
    (Utilities|SpawnWave))
  (if (Math|Conversions|ToBoolean(Integer) (+ (Utilities|Array|Length (Variables|Default|GetQueuedEnemies)) (Utilities|Array|Length (Variables|Default|GetAliveEnemies))))
    _
    (else
      (Variables|/Script/MyProject.WaveManager|SetbM_WaveEnded (Variables|Default|GetWaveManager) true)))
  ;[1 1 1] Remove dead enemies
  (for (_array_element _array_index) (Variables|Default|GetAliveEnemies)
    (Utilities|IsValid _array_element
      (:Is%20Not%20Valid
        (Utilities|Array|RemoveIndex (Variables|Default|GetAliveEnemies) _array_index))))
  (Utilities|CheckWinandLose
    (:Win
      ;[1 1 1] Victory/lose
      (if (not (Variables|Default|GetAlreadyDisabled))
        (CallFunction|DisableAll)
        (Audio|SpawnSound2D "/Game/Sounds/SFX_Victory.SFX_Victory" 1.0 1.0 0.0 0)))
    (:Lose
      (if (not (Variables|Default|GetAlreadyDisabled))
        (CallFunction|DisableAll)))
    (:Neither
      (if (and (not (Variables|Default|GetAppliedMoney)) (Variables|/Script/MyProject.WaveManager|GetbM_WaveEnded (Variables|Default|GetWaveManager)))
        (Variables|/Game/Blueprints/BP_GameInstance.BP_GameInstance_C|SetCoins _gameinstance (+ (.wavewinmoneyreward (Variables|Default|GetCurrentWave)) (Variables|/Game/Blueprints/BP_GameInstance.BP_GameInstance_C|GetCoins _gameinstance)))
        (Variables|Default|SetAppliedMoney true)))))

(fn ConstructionScript)