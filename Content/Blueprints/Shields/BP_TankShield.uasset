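; BP_TankShield is the tank shield variant of a parent shield Blueprint.
; It copies TankShieldMaxHealth into MaxHealth on both BeginPlay and Initialize, before calling the parent logic.
; After parent initialization it sets the nav modifier area type to BPNA_TankShield, giving the shield its own navigation area class.
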(event EventBeginPlay
  (Variables|Default|SetMaxHealth (Variables|Default|GetTankShieldMaxHealth))
  (|CallParentFunction))

(event Collision|EventActorBeginOverlap
  (params (OtherActor :type Actor%20Object%20Reference))
  (|CallParentFunction OtherActor) ; This node is disabled and will not be called.\nDrag off pins to build functionality.
)

(event EventTick
  (params (DeltaSeconds :type Float%20%28single-precision%29))
  (|CallParentFunction DeltaSeconds) ; This node is disabled and will not be called.\nDrag off pins to build functionality.
)

(fn ConstructionScript
  (|CallParentFunction))

(fn Initialize
  (Variables|Default|SetMaxHealth (Variables|Default|GetTankShieldMaxHealth))
  (|CallParentFunction)
  (Variables|Default|SetNavModiferAreaType "/Game/Blueprints/Shields/BPNA_TankShield.BPNA_TankShield_C"))