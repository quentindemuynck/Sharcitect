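; BP_ShieldManager is an actor that keeps a registry of shields in its Shields collection.
; AddShields adds only valid shields that are not already listed, and RemoveShields takes out valid shields that are present.
; The event graph and construction script are empty, so the registry changes only when these functions are called.
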(event EventBeginPlay)

(event Collision|EventActorBeginOverlap
  (params (OtherActor :type Actor%20Object%20Reference)))

(event EventTick
  (params (DeltaSeconds :type Float%20%28single-precision%29)))

(fn ConstructionScript)

(fn RemoveShields
  (params (Shield :type BP%20Base%20Shield%20Object%20Reference))
  (bind _shields (Variables|Default|GetShields))
  (Utilities|IsValid Shield
    (:Is%20Valid
      (if (Utilities|Array|ContainsItem _shields Shield)
        (Utilities|Array|RemoveItem _shields Shield)))))

(fn AddShields
  (params (NewShield :type BP%20Base%20Shield%20Object%20Reference))
  (bind _shields (Variables|Default|GetShields))
  (Utilities|IsValid NewShield
    (:Is%20Valid
      (if (not (Utilities|Array|ContainsItem _shields NewShield))
        (Utilities|Array|Add _shields NewShield)))))