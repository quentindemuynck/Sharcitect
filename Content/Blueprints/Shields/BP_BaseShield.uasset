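; Base placeable shield that the player buys with coins to block enemies.
; Until placed, it snaps to the mouse-nearest BP_AllowedShieldPlace, sliding along that box while placement is valid, with a green or red overlay showing validity.
; ShouldEnable deducts the price, activates collision and the nav modifier, and makes enemy AI controllers search for blocking shields.
; BPCHealth drives its health bar; destruction handling unregisters it from BP_ShieldManager and refreshes enemy targets.
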(event Custom|OnDestroyed_Event
  (params (DestroyedActor :type Actor%20Object%20Reference))
  ;[1 1 1] on destroy
  (EventDispatchers|BindEventtoOnDestroyed (delegate Custom|OnDestroyed_Event))
  (Default|RemoveShields (Variables|Default|GetShieldManager) self)
  (bind _outactors (Actor|GetAllActorsOfClass "/Game/Blueprints/Enemies/BP_BaseEnemy.BP_BaseEnemy_C"))
  (for _array_element _outactors
    (bind _asaic_base_enemy (Utilities|Casting|CastToAIC_BaseEnemy (Pawn|GetController _array_element)))
    (Default|RemoveShieldsfromBlockingShields _asaic_base_enemy)
    (Actor|DestroyActor)
    (Default|FindBlockingShields _asaic_base_enemy)))

(event EventBeginPlay
  (CallFunction|Initialize)
  (Variables|Default|SetPlayerController (Game|GetPlayerController 0))
  (bind _outactors (Actor|GetAllActorsOfClass "/Game/Blueprints/BP_AllowedShieldPlace.BP_AllowedShieldPlace_C"))
  (Variables|Default|SetAllowedShieldPlace _outactors))

(event EventTick
  (params (DeltaSeconds :type Float%20%28single-precision%29))
  (bind _returnvalue (Transformation|GetActorLocation))
  ;[1 1 1] Tick
  (if (Variables|Default|GetEnabled)
    (Transformation|SetActorLocation (Math|Vector|MakeVector (.x _returnvalue) (.y _returnvalue) (Variables|Default|GetZValue)) false false)
    (CallFunction|UpdateHealthBar)
    (if (Default|IsDead (Variables|Default|GetBPC_Health))
      (CallFunction|OnDestroyedEvent))
    (else
      ;[1 1 1] valid placing location
      (if (Variables|Default|GetIsValidPlacement)
        ;[1 1 1] Follow cursor
        (Utilities|PlacingLocationOverlay :!label _label)
        (CallFunction|ClosestShieldPlacetoMouse)
        (else
          (goto _label Exec2))))))

(fn ConstructionScript)

(fn UpdateHealthBar
  ;[1 1 1] Cast to the widget
  (bind _aswb_health_bar (Utilities|Casting|CastToWB_HealthBar (UserInterface|GetWidget (Variables|Default|GetHealth%20Bar))))
  (Progress|SetPercent (Variables|/Game/Blueprints/Damagable/WB_HealthBar.WB_HealthBar_C|GetHealthBar _aswb_health_bar) (Default|GetHealthPercentage (Variables|Default|GetBPC_Health))))

(fn Initialize
  (bind _returnvalue (Actor|GetActorOfClass "/Game/Blueprints/Shields/BP_ShieldManager.BP_ShieldManager_C"))
  (bind _output_get (Variables|Default|SetShieldManager _returnvalue))
  (Default|AddShields _output_get self)
  (Variables|/Game/Blueprints/Damagable/BPC_Health.BPC_Health_C|SetMaxHealth (Variables|Default|GetBPC_Health) (Variables|Default|GetMaxHealth))
  (CallFunction|UpdateHealthBar)
  (Default|ResetHealth (Variables|Default|GetBPC_Health))
  (bind _asbp_game_instance (Utilities|Casting|CastToBP_GameInstance (Game|GetGameInstance))
    (:then
      (Variables|Default|SetGameInstance _asbp_game_instance))
    (:CastFailed
      _))
  (Variables|Default|SetNavModiferAreaType "/Game/Blueprints/Shields/BPNA_BasicShield.BPNA_BasicShield_C")
  (CallFunction|Activate false)
  (return))

(fn ShouldEnable
  (bind _gameinstance (Variables|Default|GetGameInstance))
  (if (and (not (Variables|Default|GetEnabled)) (Variables|Default|GetIsValidPlacement))
    (Audio|SpawnSound2D "/Game/Sounds/SFX_Build.SFX_Build" 1.0 1.0 0.0 0)
    (Variables|Default|SetEnabled true)
    (for _array_element (Actor|GetComponentsByClass "/Script/Engine.StaticMeshComponent")
      (Rendering|Material|SetOverlayMaterial _array_element 0 :!class /Script/Engine.MeshComponent))
    (Variables|/Game/Blueprints/BP_GameInstance.BP_GameInstance_C|SetCoins _gameinstance (- (Variables|/Game/Blueprints/BP_GameInstance.BP_GameInstance_C|GetCoins _gameinstance) (Variables|Default|GetPrice)))
    (CallFunction|Activate true)
    (bind _outactors (Actor|GetAllActorsOfClass "/Game/Blueprints/Enemies/BP_BaseEnemy.BP_BaseEnemy_C"))
    (for _array_element_2 _outactors
      (bind _asaic_base_enemy (Utilities|Casting|CastToAIC_BaseEnemy (Pawn|GetController _array_element_2)))
      (Default|FindBlockingShields _asaic_base_enemy))
    (elif (not (Variables|Default|GetEnabled))
      (Audio|SpawnSound2D "/Game/Sounds/SFX_WRONG.SFX_WRONG" 1.0 1.0 0.0 0))))

(fn Activate
  (params (ShouldActivate :type Boolean))
  (if ShouldActivate
    (Class|NavModifierComponent|SetAreaClass (Variables|Default|GetNavModifier) (Variables|Default|GetNavModiferAreaType))
    (Collision|SetCollisionEnabled (Variables|Default|GetNormalHitbox) "QueryAndPhysics")
    (Collision|SetCollisionEnabled (Variables|Default|GetPlacementBox) "QueryOnly")
    (return)
    (else
      (Class|NavModifierComponent|SetAreaClass (Variables|Default|GetNavModifier) (LocalVariables|GetArea%20Class))
      (Collision|SetCollisionEnabled (Variables|Default|GetNormalHitbox) "NoCollision")
      (Collision|SetCollisionEnabled (Variables|Default|GetPlacementBox) "QueryOnly")
      (return))))

(fn ClosestShieldPlacetoMouse
  (bind _playercontroller (Variables|Default|GetPlayerController))
  (bind (_worldlocation _worlddirection) (Game|Player|ConvertMouseLocationToWorldSpace _playercontroller))
  (LocalVariables|SetTempDistance 9999999999999.0)
  (bind _outhit (Collision|BoxTraceByChannel _worldlocation (+ _worldlocation (* _worlddirection 99999.0)) "0, 0, 0" "0, 0, 0" "TraceTypeQuery2" false 0 "None"))
  (LocalVariables|SetImpactPoint (.ImpactPoint (Collision|BreakHitResult _outhit)))
  (for _array_element (Variables|Default|GetAllowedShieldPlace)
    (if (<= (Math|Vector|Distance(Vector) (Transformation|GetWorldLocation (Variables|/Game/Blueprints/BP_AllowedShieldPlace.BP_AllowedShieldPlace_C|GetBox _array_element)) (LocalVariables|GetImpactPoint)) (LocalVariables|GetTempDistance))
      (LocalVariables|SetTempDistance (Math|Vector|Distance(Vector) (Transformation|GetWorldLocation (Variables|/Game/Blueprints/BP_AllowedShieldPlace.BP_AllowedShieldPlace_C|GetBox _array_element)) (LocalVariables|GetImpactPoint)))
      (LocalVariables|SetClosestReference _array_element)))
  (if (Utilities|Operators|EqualEqual :A (Transformation|GetActorRotation (LocalVariables|GetClosestReference)) :ErrorTolerance 0.5)
    (LocalVariables|SetMinX (.x (- (Transformation|GetWorldLocation (Variables|/Game/Blueprints/BP_AllowedShieldPlace.BP_AllowedShieldPlace_C|GetBox (LocalVariables|GetClosestReference))) (Components|Box|GetScaledBoxExtent (Variables|/Game/Blueprints/BP_AllowedShieldPlace.BP_AllowedShieldPlace_C|GetBox (LocalVariables|GetClosestReference))))))
    (LocalVariables|SetMaxX (.x (+ (Components|Box|GetScaledBoxExtent (Variables|/Game/Blueprints/BP_AllowedShieldPlace.BP_AllowedShieldPlace_C|GetBox (LocalVariables|GetClosestReference))) (Transformation|GetWorldLocation (Variables|/Game/Blueprints/BP_AllowedShieldPlace.BP_AllowedShieldPlace_C|GetBox (LocalVariables|GetClosestReference))))))
    (Transformation|SetActorLocation (Math|Vector|MakeVector (Math|Float|Clamp(Float) (.x (LocalVariables|GetImpactPoint)) (LocalVariables|GetMinX) (LocalVariables|GetMaxX)) (.y (Transformation|GetActorLocation (LocalVariables|GetClosestReference))) (Variables|Default|GetZValue)) true false)
    (Transformation|SetActorRotation (Transformation|GetActorRotation (LocalVariables|GetClosestReference)))
    (return)
    (else
      (LocalVariables|SetMinY (- (.y (Transformation|GetActorLocation (LocalVariables|GetClosestReference))) (.y (Math|Transform|TransformLocation (Math|Transform|MakeTransform "0, 0, 0" (Transformation|GetActorRotation (LocalVariables|GetClosestReference))) (Components|Box|GetScaledBoxExtent (Variables|/Game/Blueprints/BP_AllowedShieldPlace.BP_AllowedShieldPlace_C|GetBox (LocalVariables|GetClosestReference)))))))
      (LocalVariables|SetMaxY (+ (.y (Transformation|GetActorLocation (LocalVariables|GetClosestReference))) (.y (Math|Transform|TransformLocation (Math|Transform|MakeTransform "0, 0, 0" (Transformation|GetActorRotation (LocalVariables|GetClosestReference))) (Components|Box|GetScaledBoxExtent (Variables|/Game/Blueprints/BP_AllowedShieldPlace.BP_AllowedShieldPlace_C|GetBox (LocalVariables|GetClosestReference)))))))
      (Transformation|SetActorLocation (Math|Vector|MakeVector (.x (Transformation|GetActorLocation (LocalVariables|GetClosestReference))) (Math|Float|Clamp(Float) (.y (LocalVariables|GetImpactPoint)) (LocalVariables|GetMinY) (LocalVariables|GetMaxY)) (Variables|Default|GetZValue)) true false)
      (Transformation|SetActorRotation (Transformation|GetActorRotation (LocalVariables|GetClosestReference)))
      (return))))