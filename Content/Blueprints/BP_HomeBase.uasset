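; BP_HomeBase is a base actor with a health component and a widget health bar that can be destroyed.
; UpdateHealthBar casts the HealthBar widget to WB_HealthBar and sets its percent from BPC_Health, running on BeginPlay and polling every Tick.
; When the health component fires OnDeath, the base spawns an explosion Niagara effect and sound, then hides the Cylinder and its children without destroying the actor.
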(event OnDeath(BPC_Health)
  (Niagara|SpawnSystematLocation "/Game/NiagraSystem/NS_BaseExplodes.NS_BaseExplodes" (.location (Transformation|GetActorTransform)))
  (Audio|SpawnSoundAttached "/Game/Sounds/SFX_Explosion.SFX_Explosion" (Variables|Default|GetCylinder) "None" "0, 0, 0" "0, 0, 0" "KeepRelativeOffset" false 1.0 1.0 0.0 0 0)
  (Rendering|SetVisibility (Variables|Default|GetCylinder) false true))

(event EventBeginPlay
  (CallFunction|UpdateHealthBar))

(event Collision|EventActorBeginOverlap
  (params (OtherActor :type Actor%20Object%20Reference)))

(event EventTick
  (params (DeltaSeconds :type Float%20%28single-precision%29))
  (CallFunction|UpdateHealthBar))

(fn ConstructionScript)

(fn UpdateHealthBar
  ;[1 1 1] Cast to the widget
  (bind _aswb_health_bar (Utilities|Casting|CastToWB_HealthBar (UserInterface|GetWidget (Variables|Default|GetHealthBar))))
  (Progress|SetPercent (Variables|/Game/Blueprints/Damagable/WB_HealthBar.WB_HealthBar_C|GetHealthBar _aswb_health_bar) (Default|GetHealthPercentage (Variables|Default|GetBPC_Health))))