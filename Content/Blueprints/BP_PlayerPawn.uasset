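; BP_PlayerPawn is a camera pawn that pans and scrolls over a bounded map.
; Each tick it applies consumed movement input as a world offset, using MovementSpeed for X/Y and ScrollSpeed for Z.
; CalculateMinAndMax derives X/Y limits from height, camera FOV, aspect ratio and map dimensions, so bounds follow the visible area.
; Tick then clamps the location, mapping map height to world X and width to world Y.
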(event EventBeginPlay
  (Class|CameraComponent|SetAspectRatio (Variables|Default|GetCamera) (Variables|Default|GetAspect%20Ratio)))

(event Collision|EventActorBeginOverlap
  (params (OtherActor :type Actor%20Object%20Reference)))

(event EventTick
  (params (DeltaSeconds :type Float%20%28single-precision%29))
  (bind _returnvalue (Transformation|GetActorLocation))
  (bind _movementspeed (Variables|PlayerMovement|GetMovementSpeed))
  ;[0 0.01177 1] Apply the movement
  (bind _returnvalue_2 (Class|Pawn|ConsumeMovementInputVector))
  (Transformation|AddActorWorldOffset (Math|Vector|MakeVector (* (.x (* _returnvalue_2 DeltaSeconds)) _movementspeed) (* _movementspeed (.y (* _returnvalue_2 DeltaSeconds))) (* (.z (* _returnvalue_2 DeltaSeconds)) (Variables|PlayerMovement|GetScrollSpeed))))
  (CallFunction|CalculateMinandMax)
  (Transformation|SetActorLocation (Math|Vector|MakeVector (Math|Float|Clamp(Float) (.x _returnvalue) (Variables|Default|GetMinY) (Variables|Default|GetMaxY)) (Math|Float|Clamp(Float) (.y _returnvalue) (Variables|Default|GetMinX) (Variables|Default|GetMaxX)) (Math|Float|Clamp(Float) (.z _returnvalue) (Variables|Default|GetMinZ) (Variables|Default|GetMaxZ))) false true))

(fn ConstructionScript)

(fn CalculateMinandMax
  (Variables|Default|SetHalf%20VisibleHeight (* (.z (Transformation|GetActorLocation)) (Math|Trig|Tan(Degrees) (/ (Variables|/Script/Engine.CameraComponent|GetFieldOfView (Variables|Default|GetCamera)) 2.0))))
  (Variables|Default|SetHalf%20VisibleWidth (* (Variables|Default|GetHalf%20VisibleHeight) (Variables|Default|GetAspect%20Ratio)))
  (Variables|Default|SetMinX (+ (- (.x (Variables|Default|GetMapCenter)) (/ (Variables|Default|GetMapWidth) 2.0)) (/ (Variables|Default|GetHalf%20VisibleWidth) 2.0)))
  (Variables|Default|SetMaxX (- (+ (.x (Variables|Default|GetMapCenter)) (/ (Variables|Default|GetMapWidth) 2.0)) (/ (Variables|Default|GetHalf%20VisibleWidth) 2.0)))
  (Variables|Default|SetMinY (+ (- (.y (Variables|Default|GetMapCenter)) (/ (Variables|Default|GetMapHeight) 2.0)) (/ (Variables|Default|GetHalf%20VisibleHeight) 2.0)))
  (Variables|Default|SetMaxY (- (+ (.y (Variables|Default|GetMapCenter)) (/ (Variables|Default|GetMapHeight) 2.0)) (/ (Variables|Default|GetHalf%20VisibleHeight) 2.0))))