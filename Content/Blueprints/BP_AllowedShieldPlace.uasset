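; BP_AllowedShieldPlace is a zone actor that marks where shields may be placed, allowing placement only while no enabled shield occupies it.
; Box overlap events maintain a list of BP_BaseShield actors, prune invalid entries and recalculate whether any listed shield is enabled.
; Tick writes the inverse of that occupied flag into IsValidPlacement on every listed shield, while the flag itself updates only on overlap changes.
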(event OnComponentBeginOverlap(Box)
  (params (OverlappedComponent :type Primitive%20Component%20Object%20Reference) (OtherActor :type Actor%20Object%20Reference) (OtherComp :type Primitive%20Component%20Object%20Reference) (OtherBodyIndex :type Integer) (bFromSweep :type Boolean) (SweepResult :type Hit%20Result%20Structure%20%28by%20ref%29))
  (bind _asbp_base_shield (Utilities|Casting|CastToBP_BaseShield OtherActor))
  (Utilities|Array|Add (Variables|Default|GetShields) _asbp_base_shield)
  (CallFunction|CalculateIsHoldingShield))

(event OnComponentEndOverlap(Box)
  (params (OverlappedComponent :type Primitive%20Component%20Object%20Reference) (OtherActor :type Actor%20Object%20Reference) (OtherComp :type Primitive%20Component%20Object%20Reference) (OtherBodyIndex :type Integer))
  (bind _asbp_base_shield (Utilities|Casting|CastToBP_BaseShield OtherActor))
  (Utilities|Array|RemoveItem (Variables|Default|GetShields) _asbp_base_shield)
  (CallFunction|CalculateIsHoldingShield))

(event EventBeginPlay)

(event Collision|EventActorBeginOverlap
  (params (OtherActor :type Actor%20Object%20Reference)))

(event EventTick
  (params (DeltaSeconds :type Float%20%28single-precision%29))
  (for _array_element (Variables|Default|GetShields)
    (Variables|/Game/Blueprints/Shields/BP_BaseShield.BP_BaseShield_C|SetIsValidPlacement _array_element (not (Variables|Default|GetIsHoldingShield)))))

(fn ConstructionScript)

(fn CalculateIsHoldingShield
  (CallFunction|DoesStillExists)
  (for _array_element (Variables|Default|GetShields)
    (if (Variables|/Game/Blueprints/Shields/BP_BaseShield.BP_BaseShield_C|GetEnabled _array_element)
      (Variables|Default|SetIsHoldingShield true)
      (return)))
  (Variables|Default|SetIsHoldingShield false)
  (return))

(fn DoesStillExists
  (for (_array_element _array_index) (Variables|Default|GetShields)
    (Utilities|IsValid _array_element
      (:Is%20Not%20Valid
        (Utilities|Array|RemoveIndex (Variables|Default|GetShields) _array_index))))
  (return))