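; AI controller for base enemies that runs their behavior tree to attack the base or shields blocking the way.
; On possess, it stores the base location and line-traces each nav path segment once to collect blocking shields.
; Tick drops invalid shields and feeds the Blackboard the first remaining shield's location, setting shield or base attack flags after a delay when within range.
; The controller destroys itself on unpossess.
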(event EventBeginPlay)

(event EventTick
  (params (DeltaSeconds :type Float%20%28single-precision%29))
  (CallFunction|RemoveShieldsfromBlockingShields)
  (if (Utilities|Array|IsEmpty (Variables|Shield|GetBlockingShields))
    ;[1 1 1] No Shields blocking clear the value
    (AI|Components|Blackboard|ClearValue (Variables|Default|GetBlackboard) (Variables|Shield|GetShieldLocation%20Key))
    (if (<= (Math|Vector|Distance(Vector) (AI|Components|Blackboard|GetValueasVector (Variables|Default|GetBlackboard) (Variables|Default|GetBaseLocation%20Key)) (Transformation|GetActorLocation (Variables|Default|GetPossessed%20Pawn))) (Variables|Default|GetAllowedDistanceToTarget))
      (Utilities|FlowControl|Delay 3.0)
      (AI|Components|Blackboard|SetValueasBool (Variables|Default|GetBlackboard) (Variables|Default|GetShouldAttackBase%20Key) true)
      (else
        (AI|Components|Blackboard|SetValueasBool (Variables|Default|GetBlackboard) (Variables|Default|GetShouldAttackBase%20Key) false)))
    (else
      (if (Utilities|IsShieldDifferent)
        (Utilities|AddBlockingShieldKey))
      ;[1 1 1] Add velocity
      (AI|Components|Blackboard|SetValueasFloat (Variables|Default|GetBlackboard) (Variables|Default|GetVelocityKey) (Math|Vector|VectorLength (Transformation|GetVelocity (Pawn|GetControlledPawn))))
      (if (<= (Math|Vector|Distance(Vector) (AI|Components|Blackboard|GetValueasVector (Variables|Default|GetBlackboard) (Variables|Shield|GetShieldLocation%20Key)) (Transformation|GetActorLocation (Variables|Default|GetPossessed%20Pawn))) (Variables|Default|GetAllowedDistanceToTarget))
        (Utilities|FlowControl|Delay 3.0)
        (AI|Components|Blackboard|SetValueasBool (Variables|Default|GetBlackboard) (Variables|Shield|GetShouldAttackShield%20Key) true)
        (else
          (AI|Components|Blackboard|SetValueasBool (Variables|Default|GetBlackboard) (Variables|Shield|GetShouldAttackShield%20Key) false))))))

(event EventPossess
  (params (PossessedPawn :type Pawn%20Object%20Reference))
  (Variables|Default|SetPossessed%20Pawn PossessedPawn)
  (bind _returnvalue (Actor|GetActorOfClass "/Game/Blueprints/Shields/BP_ShieldManager.BP_ShieldManager_C"))
  (Variables|Shield|SetShieldManager _returnvalue)
  ;[0.02805 0.01151 1] Move towards base
  (AI|RunBehaviorTree "/Game/Blueprints/Enemies/BT_BaseEnemy.BT_BaseEnemy")
  (bind _returnvalue_2 (Actor|GetActorOfClass "/Game/Blueprints/BP_BasePosition.BP_BasePosition_C"))
  (Variables|Default|SetBaseLocation (Transformation|GetWorldLocation (Variables|/Game/Blueprints/BP_BasePosition.BP_BasePosition_C|GetDefaultSceneRoot _returnvalue_2)))
  (AI|Components|Blackboard|SetValueasVector (Variables|Default|GetBlackboard) (Variables|Default|GetBaseLocation%20Key) (Transformation|GetWorldLocation (Variables|/Game/Blueprints/BP_BasePosition.BP_BasePosition_C|GetDefaultSceneRoot _returnvalue_2)))
  (bind _returnvalue_3 (Actor|GetActorOfClass "/Game/Blueprints/BP_HomeBase.BP_HomeBase_C"))
  (Variables|Default|SetBaseActor _returnvalue_3)
  (CallFunction|FindBlockingShields))

(event EventUnPossess
  (params (UnpossessedPawn :type Pawn%20Object%20Reference))
  (Actor|DestroyActor))

(fn ConstructionScript)

(fn FindBlockingShields
  (Utilities|Array|Clear (Variables|Shield|GetBlockingShields))
  (Utilities|Array|Add (LocalVariables|GetObject%20Types) "ObjectTypeQuery9")
  (bind _returnvalue (Class|NavigationSystemV1|FindPathtoLocationSynchronously (Pawn|GetNavAgentLocation (Variables|Default|GetPossessed%20Pawn)) (Variables|Default|GetBaseLocation) 0 (Variables|Default|GetNavQueryFilter)))
  (Utilities|IsValid _returnvalue
    (:Is%20Valid
      (bind _output_get (LocalVariables|SetPath%20Points (Variables|/Script/NavigationSystem.NavigationPath|GetPathPoints _returnvalue)))
      (for (_array_element _array_index) _output_get
        (if (Utilities|Array|IsValidIndex (LocalVariables|GetPath%20Points) (+ _array_index 1))
          (bind _outhit (Collision|LineTraceForObjects _array_element (Utilities|Array|Get(acopy) (LocalVariables|GetPath%20Points) (+ _array_index 1)) (LocalVariables|GetObject%20Types) false 0 "None"))
          ;[1 1 1] Add shield to the array if it collides with the path
          (bind _asbp_base_shield (Utilities|Casting|CastToBP_BaseShield (.HitActor (Collision|BreakHitResult _outhit))))
          (if (not (Utilities|Array|ContainsItem (Variables|Shield|GetBlockingShields) _asbp_base_shield))
            (Utilities|Array|Add (Variables|Shield|GetBlockingShields) _asbp_base_shield)))))))

(fn RemoveShieldsfromBlockingShields
  ;[0.001142 0 1] Removes non existing shields from the blocking shields
  (for _array_element (Variables|Shield|GetBlockingShields)
    (Utilities|IsValid _array_element
      (:Is%20Not%20Valid
        (Utilities|Array|RemoveItem (Variables|Shield|GetBlockingShields) _array_element)))))