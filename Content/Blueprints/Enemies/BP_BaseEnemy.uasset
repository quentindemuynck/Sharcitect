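; Base enemy character with health, a floating health bar, shooting, and a coin reward on death.
; Tick refreshes the health bar from the health component and pauses the walking sound when movement speed is low.
; Shoot spawns an enemy bullet aimed at a given target, passing damage and sound.
; On death it plays a sound, adds coins to the cached game instance and destroys itself.
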(event OnDeath(BPC_Health)
  (bind _gameinstance (Variables|Default|GetGameInstance))
  (Audio|SpawnSoundAttached "/Game/Sounds/SC_Death.SC_Death" (Variables|Collision|GetCapsuleComponent) "None" "0, 0, 0" "0, 0, 0" "KeepRelativeOffset" false 1.0 1.0 0.0 0 0)
  ;[1 1 1] Add Coins
  (Variables|/Game/Blueprints/BP_GameInstance.BP_GameInstance_C|SetCoins _gameinstance (+ (Variables|Default|GetCoinsGain) (Variables|/Game/Blueprints/BP_GameInstance.BP_GameInstance_C|GetCoins _gameinstance)))
  (Actor|DestroyActor))

(event EventBeginPlay
  (CallFunction|Initialize))

(event EventTick
  (params (DeltaSeconds :type Float%20%28single-precision%29))
  (CallFunction|UpdateHealthBar)
  ;[1 1 1] pause soond if not moving
  (Math|Float|CompareFloat (Math|Vector|VectorLength (Pawn|Components|CharacterMovement|GetLastUpdateVelocity (Variables|Character|GetCharacterMovement))) 2e+01
    (:>
      (Class|AudioComponent|SetPaused (Variables|Default|GetWalking) false))
    (:==
      (Class|AudioComponent|SetPaused (Variables|Default|GetWalking) true :!label _label))
    (:<
      (goto _label))))

(fn ConstructionScript)

(fn UpdateHealthBar
  ;[1 1 1] Cast to the widget
  (bind _aswb_health_bar (Utilities|Casting|CastToWB_HealthBar (UserInterface|GetWidget (Variables|Default|GetHealth%20Bar%20Widget))))
  (Progress|SetPercent (Variables|/Game/Blueprints/Damagable/WB_HealthBar.WB_HealthBar_C|GetHealthBar _aswb_health_bar) (Default|GetHealthPercentage (Variables|Default|GetBPC_Health))))

(fn Shoot
  (params (ShootTarget :type Actor%20Object%20Reference))
  (Variables|Default|SetShoot%20Target ShootTarget)
  (Utilities|IsValid ShootTarget
    (:Is%20Valid
      (Game|SpawnActorfromClass "/Game/Blueprints/Enemies/BP_EnemyBullet.BP_EnemyBullet_C" (Math|Transform|MakeTransform (Transformation|GetWorldLocation (Variables|Default|GetBullet%20Spawn%20Pos)) (Math|Conversions|RotationFromXVector (Math|Vector|GetUnitDirection(Vector) (Transformation|GetWorldLocation (Variables|Default|GetBullet%20Spawn%20Pos)) (Transformation|GetActorLocation (Variables|Default|GetShoot%20Target)))) "1.000000,1.000000,1.000000") "Undefined" "MultiplyWithRoot" 0 ShootTarget (Variables|Default|GetDamage) "/Game/Sounds/SC_BasicBullet.SC_BasicBullet" 0))))

(fn Initialize
  (CallFunction|UpdateHealthBar)
  (bind _asbp_game_instance (Utilities|Casting|CastToBP_GameInstance (Game|GetGameInstance)))
  (Variables|Default|SetGameInstance _asbp_game_instance)
  (return))