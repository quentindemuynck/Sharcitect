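; Shield healer turret, a child Blueprint that targets BP_BaseShield actors and fires healing shots at them.
; It reuses the parent's turret logic, loading healing stats into its range, damage and fire-delay variables and always selecting a new target.
; Retargeting removes disabled shields from the inherited Enemies list and defers to the parent's selection.
; Each shot spawns a BP_ShieldBullet toward the target with health VFX and a limited lifespan.
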(event EventBeginPlay
  (Variables|Default|SetRange (Variables|Default|GetHealing%20Range))
  (|CallParentFunction)
  (Variables|Default|SetTargetClass "/Game/Blueprints/Shields/BP_BaseShield.BP_BaseShield_C")
  (Variables|Default|SetDamage (Variables|Default|GetHealing))
  (Variables|Default|SetShotDelay (Variables|Default|GetShootSpeedHealer))
  (Variables|Default|SetAlwaysSelectNewTarget true)
  (Variables|Default|SetTargetType (Variables|Default|GetTarget%20Type))
  (Variables|Default|SetName (Variables|Default|GetShieldHealerName))
  (Variables|Default|SetPrice (Class|KismetMathLibrary|ToInt64(Integer) (Variables|Default|GetShieldHealerPrice))))

(event Collision|EventActorBeginOverlap
  (params (OtherActor :type Actor%20Object%20Reference)))

(event EventTick
  (params (DeltaSeconds :type Float%20%28single-precision%29))
  (|CallParentFunction DeltaSeconds) ; This node is disabled and will not be called.\nDrag off pins to build functionality.
)

(fn ConstructionScript
  (|CallParentFunction))

(fn ShootBullet
  (bind _target (Variables|Default|GetTarget))
  (Utilities|IsValid _target
    (:Is%20Valid
      (bind _returnvalue (Game|SpawnActorfromClass "/Game/Blueprints/Turrets/BP_ShieldBullet.BP_ShieldBullet_C" (Math|Transform|MakeTransform (Transformation|GetWorldLocation (Variables|Default|GetBulletSpawnPos)) (Math|Conversions|RotationFromXVector (Variables|Default|GetAimingDirection)) "1.000000,1.000000,1.000000") "Undefined" "MultiplyWithRoot" 0 _target (Variables|Default|GetDamage) "/Game/Sounds/SC_BasicBullet.SC_BasicBullet" "/Game/NiagraSystem/NS_Health.NS_Health" 0))
      (Actor|SetLifeSpan _returnvalue 1e+01))))

(fn Initialize
  (Variables|Default|SetRange (Variables|Default|GetHealing%20Range))
  (|CallParentFunction)
  (Variables|Default|SetTargetClass "/Game/Blueprints/Shields/BP_BaseShield.BP_BaseShield_C")
  (Variables|Default|SetDamage (Variables|Default|GetHealing))
  (Variables|Default|SetShotDelay (Variables|Default|GetShootSpeedHealer))
  (Variables|Default|SetAlwaysSelectNewTarget true)
  (Variables|Default|SetTargetType (Variables|Default|GetTarget%20Type))
  (Variables|Default|SetName (Variables|Default|GetShieldHealerName))
  (Variables|Default|SetPrice (Class|KismetMathLibrary|ToInt64(Integer) (Variables|Default|GetShieldHealerPrice))))

(fn SetNewTarget
  (for (_array_element _array_index) (Variables|Default|GetEnemies)
    (bind _asbp_base_shield (Utilities|Casting|CastToBP_BaseShield _array_element)
      (:then
        (if (not (Variables|/Game/Blueprints/Shields/BP_BaseShield.BP_BaseShield_C|GetEnabled _asbp_base_shield))
          (Utilities|Array|RemoveIndex (Variables|Default|GetEnemies) _array_index)))
      (:CastFailed
        (|CallParentFunction))))
  (|CallParentFunction))