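; BP_MagicalTower is the magic turret variant, a child Blueprint that feeds its magic-specific stats into a parent turret class.
; Initialize copies range, damage, fire delay, target type, name and price into shared variables, with range stored in FlameRange before the parent initialization runs.
; ShootBullet spawns a BP_MagicBullet at the muzzle along the aiming direction, passing it the target and damage when the target is valid.
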(event Collision|EventActorBeginOverlap
  (params (OtherActor :type Actor%20Object%20Reference))
  (|CallParentFunction OtherActor) ; This node is disabled and will not be called.\nDrag off pins to build functionality.
)

(event EventTick
  (params (DeltaSeconds :type Float%20%28single-precision%29))
  (|CallParentFunction DeltaSeconds))

(event EventBeginPlay
  (Variables|Default|SetFlameRange (Variables|Default|GetMagicRange))
  (|CallParentFunction)
  (CallFunction|Initialize))

(fn ConstructionScript
  (|CallParentFunction))

(fn Initialize
  (Variables|Default|SetFlameRange (Variables|Default|GetMagicRange))
  (|CallParentFunction)
  (Variables|Default|SetDamage (Variables|Default|GetMagicDamage))
  (Variables|Default|SetShotDelay (Variables|Default|GetMagicShootingSpeed))
  (Variables|Default|SetTargetType (Variables|Default|GetMagicTargetType))
  (Variables|Default|SetName (Variables|Default|GetMagicTurretName))
  (Variables|Default|SetPrice (Variables|Default|GetMagicTurretPrice)))

(fn ShootBullet
  (bind _target (Variables|Default|GetTarget))
  (Utilities|IsValid _target
    (:Is%20Valid
      (Game|SpawnActorfromClass "/Game/Blueprints/Turrets/BP_MagicBullet.BP_MagicBullet_C" (Math|Transform|MakeTransform (Transformation|GetWorldLocation (Variables|Default|GetBulletSpawnPos)) (Math|Conversions|RotationFromXVector (Variables|Default|GetAimingDirection)) "1.000000,1.000000,1.000000") "Undefined" "MultiplyWithRoot" 0 _target (Variables|Default|GetMagicDamage) 0))))