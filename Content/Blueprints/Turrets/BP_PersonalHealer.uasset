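; BP_PersonalHealer is the Personal Healer turret, a child Blueprint that configures inherited turret logic for healing.
; Initialize copies PersonalHealer values into name, price, shot delay and target type, stores the healing amount in Damage, and forces a new target selection each time.
; HealingRange is set before the parent call in both BeginPlay and Initialize, leaving targeting and firing behavior to the parent.
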(event EventBeginPlay
  (Variables|Default|SetHealing%20Range (Variables|Default|GetPersonalHealerRange))
  (|CallParentFunction))

(event Collision|EventActorBeginOverlap
  (params (OtherActor :type Actor%20Object%20Reference))
  (|CallParentFunction OtherActor) ; This node is disabled and will not be called.\nDrag off pins to build functionality.
)

(event EventTick
  (params (DeltaSeconds :type Float%20%28single-precision%29))
  (|CallParentFunction DeltaSeconds) ; This node is disabled and will not be called.\nDrag off pins to build functionality.
)

(fn ConstructionScript
  (|CallParentFunction))

(fn Initialize
  (Variables|Default|SetHealing%20Range (Variables|Default|GetPersonalHealerRange))
  (|CallParentFunction)
  (Variables|Default|SetName (Variables|Default|GetPersonalHealerName))
  (Variables|Default|SetPrice (Variables|Default|GetPersonalHealerPrice))
  (Variables|Default|SetDamage (Variables|Default|GetPersonalHealerHealing))
  (Variables|Default|SetShotDelay (Variables|Default|GetPersonalHealerSpeed))
  (Variables|Default|SetAlwaysSelectNewTarget true)
  (Variables|Default|SetTargetType (Variables|Default|GetPersonalHealerTargetType)))