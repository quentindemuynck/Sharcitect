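; BP_MagicBullet is a magic projectile variant for turrets, built on a parent class that supplies the base bullet behavior.
; On BeginPlay it assigns its own sound cue, runs the parent logic, sets its lifespan from MagicLifeSpan and selects a blood Niagara effect.
; On overlap it runs the parent handling, then resets its lifespan to a short fixed delay before destruction.
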(event EventBeginPlay
  (Variables|Default|SetBulletSounds "/Game/Sounds/SC_MagicBullet.SC_MagicBullet")
  (|CallParentFunction)
  (Actor|SetLifeSpan (Variables|Default|GetMagicLifeSpan))
  (Variables|Default|SetNiagaraSystem "/Game/NiagraSystem/NS_Blood.NS_Blood"))

(event Collision|EventActorBeginOverlap
  (params (OtherActor :type Actor%20Object%20Reference))
  (|CallParentFunction OtherActor)
  (Actor|SetLifeSpan 0.9))

(event EventTick
  (params (DeltaSeconds :type Float%20%28single-precision%29))
  (|CallParentFunction DeltaSeconds) ; This node is disabled and will not be called.\nDrag off pins to build functionality.
)

(fn ConstructionScript
  (|CallParentFunction))