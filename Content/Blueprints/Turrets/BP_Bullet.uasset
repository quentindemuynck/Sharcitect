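; Turret bullet that homes in on its Target, dealing damage through BPI_Damagable on overlap.
; With a valid Target at BeginPlay, it activates homing movement, sets a lifespan and plays an attached sound.
; Every box overlap spawns blood Niagara oriented along velocity, whether or not the hit is damageable.
; Damage goes to the hit actor, or else its implementing components, and DestroyOnHit controls whether the bullet then destroys itself.
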(event OnComponentBeginOverlap(Box)
  (params (OverlappedComponent :type Primitive%20Component%20Object%20Reference) (OtherActor :type Actor%20Object%20Reference) (OtherComp :type Primitive%20Component%20Object%20Reference) (OtherBodyIndex :type Integer) (bFromSweep :type Boolean) (SweepResult :type Hit%20Result%20Structure%20%28by%20ref%29))
  (Niagara|SpawnSystemAttached (Variables|Default|GetNiagaraSystem) OtherComp "None" "0, 0, 0" (Math|Conversions|RotationFromXVector (Variables|/Script/Engine.MovementComponent|GetVelocity (Variables|Default|GetProjectileMovement))) "SnapToTarget" true)
  (CallFunction|CheckifHitActorandDoDamage OtherActor (Variables|Default|GetDestroyOnHit)))

(event EventBeginPlay
  (bind _target (Variables|Default|GetTarget))
  (bind _projectilemovement (Variables|Default|GetProjectileMovement))
  (Variables|Default|SetNiagaraSystem "/Game/NiagraSystem/NS_Blood.NS_Blood")
  (Utilities|IsValid _target
    (:Is%20Valid
      (Variables|/Script/Engine.ProjectileMovementComponent|SetHomingTargetComponent _projectilemovement (Variables|/Script/Engine.Actor|GetRootComponent _target))
      (Components|Activation|Activate _projectilemovement false)
      (Actor|SetLifeSpan 1e+01)
      (Audio|SpawnSoundAttached (Variables|Default|GetBulletSounds) (Variables|Default|GetBox) "None" "0, 0, 0" "0, 0, 0" "KeepRelativeOffset" false 1.0 1.0 0.0 0 0))))

(fn ConstructionScript)

(fn CheckifHitActorandDoDamage
  (params (HitActor :type Actor%20Object%20Reference) (DestroyBullet :type Boolean))
  (bind _returnvalue (Class|Actor|GetComponentsbyInterface HitActor "/Game/Blueprints/Damagable/BPI_Damagable.BPI_Damagable_C"))
  (LocalVariables|SetDestroy DestroyBullet)
  ;[1 1 1] BPI_damagable on hit actor
  (Utilities|IsValid HitActor
    (:Is%20Valid
      (if (Utilities|DoesObjectImplementInterface HitActor "/Game/Blueprints/Damagable/BPI_Damagable.BPI_Damagable_C")
        (Class|BPIDamagable|DoDamage(Message) HitActor (Variables|Damage|GetDamageAmount))
        (if (LocalVariables|GetDestroy)
          (Actor|DestroyActor))
        (else
          (bind _index (Utilities|FlowControl|ForLoopwithBreak 0 (- (Utilities|Array|Length _returnvalue) 1) :!label _label)
            (:LoopBody
              (Class|BPIDamagable|DoDamage(Message) (Utilities|Array|Get(acopy) _returnvalue _index) (Variables|Damage|GetDamageAmount))
              (Utilities|IsValid HitActor
                (:Is%20Valid
                  (if (LocalVariables|GetDestroy)
                    (Actor|DestroyActor)))
                (:Is%20Not%20Valid
                  (goto _label Break))))))))))