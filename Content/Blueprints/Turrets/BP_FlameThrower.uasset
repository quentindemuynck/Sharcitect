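; BP_FlameThrower is a flamethrower turret that fires flame projectiles at its target.
; BeginPlay and Initialize both copy flamethrower-specific stats, targeting type, name and price into inherited turret variables, setting Range before the parent call and the rest after.
; ShootBullet spawns a BP_Flame at the bullet spawn point along the aiming direction when the target is valid, passing it the target, damage and sound.
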(event EventBeginPlay
  (Variables|Default|SetRange (Variables|Default|GetFlameRange))
  (|CallParentFunction)
  (Variables|Default|SetDamage (Variables|Default|GetFlameDamage))
  (Variables|Default|SetShotDelay (Variables|Default|GetFlameDelay))
  (Variables|Default|SetTargetType (Variables|Default|GetDefaultTargetType))
  (Variables|Default|SetName (Variables|Default|GetFlameThrowerName))
  (Variables|Default|SetPrice (Class|KismetMathLibrary|ToInt64(Integer) (Variables|Default|GetFlamethrowerCosts))))

(event Collision|EventActorBeginOverlap
  (params (OtherActor :type Actor%20Object%20Reference)))

(event EventTick
  (params (DeltaSeconds :type Float%20%28single-precision%29))
  (|CallParentFunction DeltaSeconds) ; This node is disabled and will not be called.\nDrag off pins to build functionality.
)

(fn ConstructionScript
  (|CallParentFunction))

(fn ShootBullet
  (bind _target (Variables|Default|GetTarget))
  (Utilities|IsValid _target
    (:Is%20Valid
      (Game|SpawnActorfromClass "/Game/Blueprints/Turrets/BP_Flame.BP_Flame_C" (Math|Transform|MakeTransform (Transformation|GetWorldLocation (Variables|Default|GetBulletSpawnPos)) (Math|Conversions|RotationFromXVector (Variables|Default|GetAimingDirection)) "1.000000,1.000000,1.000000") "Undefined" "MultiplyWithRoot" 0 _target (Variables|Default|GetDamage) "/Game/Sounds/SC_BasicBullet.SC_BasicBullet" 0))))

(fn Initialize
  (Variables|Default|SetRange (Variables|Default|GetFlameRange))
  (|CallParentFunction)
  (Variables|Default|SetDamage (Variables|Default|GetFlameDamage))
  (Variables|Default|SetShotDelay (Variables|Default|GetFlameDelay))
  (Variables|Default|SetTargetType (Variables|Default|GetDefaultTargetType))
  (Variables|Default|SetName (Variables|Default|GetFlameThrowerName))
  (Variables|Default|SetPrice (Class|KismetMathLibrary|ToInt64(Integer) (Variables|Default|GetFlamethrowerCosts))))